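; Paper2D side-scroller player character, a gunman that walks along world X and jumps from named input bindings.
; Each tick it picks the jump, run or idle flipbook from the falling state and velocity.
; It also snaps the controller yaw to face the direction of X velocity, keeping the last facing when stopped.
; Jump press and release also print debug strings.
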(event `InputAction|gunman_jump`
  (params (Key :type "Key Structure"))
  (:`Pressed`
    (`KismetSystemLibrary.PrintString` "jump")
    (`self.Jump`))
  (:`Released`
    (`KismetSystemLibrary.PrintString` "fall")
    (`self.StopJumping`)))

(event `InputAxis|gunman_walk`
  (params (AxisValue :type "Float (single-precision)"))
  (`self.AddMovementInput` (1.0 0.0 0.0) AxisValue))

(event `self.ReceiveTick`
  (params (DeltaSeconds :type "Float (single-precision)"))
  (`self.update animation`)
  (`self.update control rotation`))

(event `update animation`
  (`PaperFlipbookComponent.SetFlipbook` (`self.PaperFlipbook`) (select `bool` (`NavMovementComponent.IsFalling` (`self.CharacterMovement`)) :`false` (select `bool` (> (`KismetMathLibrary.VSize` (`MovementComponent.Velocity` (`self.CharacterMovement`))) 0.0) :`false` "/Game/nicola_h_content/character/fb_gunman_idle.fb_gunman_idle" :`true` "/Game/nicola_h_content/character/fb_gunman_run.fb_gunman_run" :!type "PaperFlipbook Object Reference") :`true` "/Game/nicola_h_content/character/fb_gunman_jump.fb_gunman_jump")))

(event `update control rotation`
  (`/Engine/EditorBlueprintResources/StandardMacros.IsValid` (`self.GetController`)
    (:`Is Valid`
      (`/Engine/EditorBlueprintResources/StandardMacros.CompareFloat` (.x (`MovementComponent.Velocity` (`self.CharacterMovement`)))
        (:`>`
          (`Controller.SetControlRotation` (`self.GetController`) (`KismetMathLibrary.MakeRotator` 0.0)))
        (:`<`
          (`Controller.SetControlRotation` (`self.GetController`) (`KismetMathLibrary.MakeRotator` 0.0 0.0 180.0)))))))

(fn `UserConstructionScript`)